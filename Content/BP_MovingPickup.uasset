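; BP_MovingPickup is an actor that continuously circles its spawn point, with no collection logic in these graphs.
; BeginPlay stores the starting location, and Tick sets the location to that point plus a sine and cosine offset scaled by Distance0.
; The orbit lies in the world YZ plane and follows unpaused game time, with no sweep.
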(event EventBeginPlay
  (|CallParentFunction)
  (Variables|Default|SetStartingPosition_0 (Transformation|GetActorLocation)))

(event Collision|EventActorBeginOverlap
  (params (OtherActor :type Actor%20Object%20Reference))
  (|CallParentFunction OtherActor) ; This node is disabled and will not be called.\nDrag off pins to build functionality.
)

(event EventTick
  (params (DeltaSeconds :type Float%20%28single-precision%29))
  (bind _returnvalue (Class|GameplayStatics|GetUnpausedTimeSeconds))
  (|CallParentFunction DeltaSeconds)
  (Transformation|SetActorLocation (+ (* (Math|Vector|MakeVector 0.0 (Math|Trig|Sin(Radians) _returnvalue) (Math|Trig|Cos(Radians) _returnvalue)) (Variables|Default|GetDistance_0)) (Variables|Default|GetStartingPosition_0)) false false))

(fn ConstructionScript
  (|CallParentFunction))