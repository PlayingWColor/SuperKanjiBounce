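; BP_Player is the player Blueprint, handling audio feedback for movement and pickup actions.
; On BeginPlay it binds jump, bounce, select, grab, drop and submit events to one-shot 2D sounds, and starts persistent wind and stage music sounds.
; Tick uses velocity magnitude to raise wind volume with speed, while music holds at half volume until mid speed, then fades out.
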(event Custom|OnBounceEvent
  (Audio|PlaySound2D "/Game/Audio/SFX/SFX_explosionShort1.SFX_explosionShort1" 1.0 1.0 0.0 0 0))

(event Custom|OnJumpEvent
  (Audio|PlaySound2D "/Game/Audio/SFX/SFX_pushLong.SFX_pushLong" 1.0 1.0 0.0 0 0))

(event Custom|OnSelectEvent
  (Audio|PlaySound2D "/Game/Audio/SFX/SFX_UIGeneric7.SFX_UIGeneric7" 1.0 1.0 0.0 0 0))

(event Custom|OnGrabPickupEvent
  (Audio|PlaySound2D "/Game/Audio/SFX/SFX_collect_bonus11.SFX_collect_bonus11" 1.0 1.0 0.0 0 0))

(event Custom|OnDropPickupEvent
  (Audio|PlaySound2D "/Game/Audio/SFX/SFX_hit_damage13.SFX_hit_damage13" 1.0 1.0 0.0 0 0))

(event Custom|OnSubmitPickupEvent
  (Audio|PlaySound2D "/Game/Audio/SFX/SFX_powerUp7.SFX_powerUp7" 1.0 1.0 0.0 0 0))

(event EventBeginPlay
  (EventDispatchers|AssignOnJump (delegate Custom|OnJumpEvent))
  (EventDispatchers|AssignOnBounce (delegate Custom|OnBounceEvent))
  (EventDispatchers|AssignOnSelect (delegate Custom|OnSelectEvent))
  (EventDispatchers|AssignOnGrabPickup (delegate Custom|OnGrabPickupEvent))
  (EventDispatchers|AssignOnDropPickup (delegate Custom|OnDropPickupEvent))
  (EventDispatchers|AssignOnSubmitPickup (delegate Custom|OnSubmitPickupEvent))
  (bind _returnvalue (Audio|SpawnSound2D "/Game/Audio/SFX/wind.wind" 0.0 1.0 0.0 0 false false))
  (Variables|Default|SetWindSFX _returnvalue)
  (bind _returnvalue_2 (Audio|SpawnSound2D "/Game/Audio/Music/CaptChipPants_loop__128_.CaptChipPants_loop__128_" 1.0 1.0 0.0 0 false false))
  (Variables|Default|SetStageMusic _returnvalue_2))

(event Collision|EventActorBeginOverlap
  (params (OtherActor :type Actor%20Object%20Reference)))

(event EventTick
  (params (DeltaSeconds :type Float%20%28single-precision%29))
  (bind _returnvalue (Transformation|GetVelocity))
  (bind _returnvalue_2 (Math|Vector|VectorLength _returnvalue))
  (bind _returnvalue_3 (/ _returnvalue_2 6e+03))
  (Audio|Components|Audio|SetVolumeMultiplier (Variables|Default|GetWindSFX) _returnvalue_3 :!class /Script/Engine.AudioComponent)
  (Audio|Components|Audio|SetVolumeMultiplier (Variables|Default|GetStageMusic) (- 1.0 (Math|Float|Clamp(Float) _returnvalue_3 0.5)) :!class /Script/Engine.AudioComponent))

(fn ConstructionScript)